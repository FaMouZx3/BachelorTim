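; Shared AR placement manager that syncs a cloud anchor between host and clients and spawns selected items relative to it.
; The host taps tracked geometry to host a Cloud AR Pin and passes its ID to the WorldAnchor.
; Clients poll for that ID on Tick, resolve the pin and align their anchor.
; Once Ready, taps become anchor-relative transforms for the server-side PlaceObject, which attaches spawned actors to the anchor.
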(event `self.ReceiveBeginPlay`
  ;[0 1 0] Initialisierung + Referenzierung
  (`KismetSystemLibrary.Delay` 0.2)
  (`/Engine/EditorBlueprintResources/ActorMacros.Switch Has Authority`
    (:`Authority`
      (set `self.States` "NewEnumerator1"))
    (:`Remote`
      (set `self.States` "NewEnumerator3")
      (bind _outactors (`GameplayStatics.GetAllActorsOfClass` "/Game/Bachelor_Tim/Blueprints/Placeable/BP_WorldAnchor.BP_WorldAnchor_C"))
      (set `self.World Anchor` (`|GetArrayItem` _outactors)))))

(event `self.ReceiveTick`
  (params (DeltaSeconds :type "Float (single-precision)"))
  ;[0 1 0] Im Tick wird geprüft ob ein Anchor angelegt wurde und ob er resolved werden kann
  (switch `/Game/Bachelor_Tim/Blueprints/GameModes/GameStates` (`self.States`)
    (:`NewEnumerator3`
      (`self.Is Cloud ID Valid?`))
    (:`NewEnumerator4`
      (`self.Resolve Cloud Anchor`))))

(event `InputTouch`
  (params (Location :type "Vector Structure") (FingerIndex :type "ETouchIndex Enum"))
  ;[0 1 0] Platzieren des Cloud Anchor auf seiten des Host und das platzieren von ausgewählten Items in der Welt
  (:`Pressed`
    (switch `/Game/Bachelor_Tim/Blueprints/GameModes/GameStates` (`self.States`)
      (:`NewEnumerator1`
        (`self.Set Cloud Anchor` FingerIndex))
      (:`NewEnumerator5`
        (`self.Place Item`)))))

(event `Place Object`
  (params (Position :type "Transform Structure"))
  ;[0 1 0] Platzieren der ausgewählten Objekte in der Welt (Wird auf dem Server ausgeführt) und wird relativ zum Cloud Anchor verschoben
  (if (!= (`self.Spawnable Actor`) null)
    (bind _returnvalue (`|SpawnActorFromClass` (`self.Spawnable Actor`) (`KismetMathLibrary.MakeTransform` (0.0 0.0 0.0)) "Undefined" "OverrideRootScale" null null))
    (`self.K2_AttachToActor` _returnvalue (`self.World Anchor`) "None" "KeepRelative" "KeepRelative" "KeepRelative" true)
    (`self.K2_SetActorRelativeTransform` _returnvalue Position false false)
    (set `self.Spawnable Actor` null)))

(fn `Get Relative Position`
  (params (`Input Transform` :type "Transform Structure"))
  (returns (`Output Transform` :type "Transform Structure"))
  (bind _returnvalue (`SceneComponent.K2_GetComponentToWorld` (`/Game/Bachelor_Tim/Blueprints/Placeable/BP_WorldAnchor.WorldAnchorRoot` (`self.World Anchor`))))
  ;[0 1 0] Hier wird die relative Position zwischen dem Tippen auf der Plane und dem platzierten World Anchor berechnet um auf Server und Client die gleichen Positionen zu bekommen (Habe mir diese Funktion von Google AR Template abgeschaut)
  (return (`KismetMathLibrary.MakeTransform` (`KismetMathLibrary.InverseTransformLocation` _returnvalue `Input Transform_Location`) (`KismetMathLibrary.InverseTransformRotation` _returnvalue `Input Transform_Rotation`))))

(fn `UserConstructionScript`)