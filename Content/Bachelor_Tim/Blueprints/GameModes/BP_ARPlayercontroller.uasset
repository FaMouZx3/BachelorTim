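; Player controller for an AR level using Google ARCore and online sessions.
; On begin play the local controller adds room-info and item-list-button widgets, starts the AR session and caches the place manager, which receives touch presses.
; Tick polls until it finds and caches the world anchor actor.
; Android Back destroys the online session and opens the start map even on failure; EndPlay stops the AR session.
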(event `self.ReceiveBeginPlay`
  (if (`self.IsLocalPlayerController`)
    (bind _returnvalue (`|CreateWidget` "/Game/Bachelor_Tim/Blueprints/UI/UI_ARRoomInformation.UI_ARRoomInformation_C" self))
    (`UserWidget.AddToViewport` _returnvalue 0)
    (bind _returnvalue_2 (`|CreateWidget` "/Game/Bachelor_Tim/Blueprints/UI/UI_ItemListButton.UI_ItemListButton_C"))
    (`UserWidget.AddToViewport` _returnvalue_2 0)
    (`GoogleARCoreServicesFunctionLibrary.ConfigGoogleARCoreServices` (make `GoogleARCoreServicesConfig` "Enabled"))
    (`ARBlueprintLibrary.StartARSession` "/Game/Bachelor_Tim/Blueprints/GameModes/ARSessionConfig.ARSessionConfig")
    (bind _outactors (`GameplayStatics.GetAllActorsOfClass` "/Game/Bachelor_Tim/Blueprints/Manager/BP_PlaceManager.BP_PlaceManager_C"))
    (set `self.Place Manager Ref` (`|GetArrayItem` _outactors))))

(event `self.ReceiveEndPlay`
  (params (EndPlayReason :type "EEndPlayReason Enum" :default "Destroyed"))
  (if (`self.IsLocalPlayerController`)
    (`ARBlueprintLibrary.StopARSession`)))

(event `Key|Android_Back`
  (params (Key :type "Key Structure"))
  (:`Pressed`
    (if (`self.IsLocalController`)
      (`DestroySessionCallbackProxy.DestroySession` self
        (:`OnSuccess`
          _)
        (:`OnFailure`
          _))
      (`GameplayStatics.OpenLevel` "StartMap"))))

(event `InputTouch`
  (params (Location :type "Vector Structure") (FingerIndex :type "ETouchIndex Enum"))
  (:`Pressed`
    (`/Game/Bachelor_Tim/Blueprints/Manager/BP_PlaceManager.Pressed` (`self.Place Manager Ref`) FingerIndex)))

(event `self.ReceiveTick`
  (params (DeltaSeconds :type "Float (single-precision)"))
  (`/Engine/EditorBlueprintResources/StandardMacros.IsValid` (`self.World Anchor Ref`)
    (:`Is Not Valid`
      (bind _outactors (`GameplayStatics.GetAllActorsOfClass` "/Game/Bachelor_Tim/Blueprints/Placeable/BP_WorldAnchor.BP_WorldAnchor_C"))
      (if (> (`KismetArrayLibrary.Array_Length` _outactors) 0)
        (set `self.World Anchor Ref` (`|GetArrayItem` _outactors))
        (`KismetSystemLibrary.PrintString` "Habe mir den World Anchor geholt")))))

(fn `UserConstructionScript`)