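; BP_WorldAnchor is an actor that keeps its WorldAnchor component aligned with a tracked AR pin.
; On BeginPlay, the authority copies the RoomID from BP_GameInstance.
; Each tick, while the Pin is valid and tracking, it sets the component's world transform to the pin's local-to-world transform.
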(event `self.ReceiveBeginPlay`
  (`/Engine/EditorBlueprintResources/ActorMacros.Switch Has Authority`
    (:`Authority`
      (bind _asbp_game_instance (cast `/Game/Bachelor_Tim/Blueprints/ServerBP/BP_GameInstance` (`GameplayStatics.GetGameInstance`)))
      (set `self.RoomID` (`/Game/Bachelor_Tim/Blueprints/ServerBP/BP_GameInstance.RoomID` _asbp_game_instance)))))

(event `self.ReceiveTick`
  (params (DeltaSeconds :type "Float (single-precision)"))
  (bind _pin (`self.Pin`))
  (if (`KismetSystemLibrary.IsValid` (`self.Pin`))
    (if (`|EnumEquality` (`ARPin.GetTrackingState` _pin) "Tracking")
      (`SceneComponent.K2_SetWorldTransform` (`self.WorldAnchor`) (`ARPin.GetLocalToWorldTransform` _pin) false false))))

(fn `UserConstructionScript`)