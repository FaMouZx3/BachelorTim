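; BP_WorldAnchor is a placeable actor that serves as the shared AR world anchor for a multiplayer session using cloud anchors.
; On BeginPlay the authority copies the room ID from BP_GameInstance.
; SetCloudID stores the cloud ID on the authority only, for replication to clients so they can resolve the anchor.
; Tick snaps the root to its AR pin's transform while tracking, correcting drift.
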(event `self.ReceiveBeginPlay`
  ;[0 1 0] Setzen der erstellten Raum ID (nur der Host, da der Client diese Information nur vom Host bekommen kann)
  (`/Engine/EditorBlueprintResources/ActorMacros.Switch Has Authority`
    (:`Authority`
      (bind _asbp_game_instance (cast `/Game/Bachelor_Tim/Blueprints/ServerBP/BP_GameInstance` (`GameplayStatics.GetGameInstance`)))
      (set `self.RoomID` (`/Game/Bachelor_Tim/Blueprints/ServerBP/BP_GameInstance.RoomID` _asbp_game_instance)))))

(event `self.ReceiveTick`
  (params (DeltaSeconds :type "Float (single-precision)"))
  (bind _pin (`self.Pin`))
  ;[0 1 0] Hier wird der World Anchor Actor auf die Ursrüngliche Cloud Anchor Transform gesetzt falls eine Verschiebung durch das AR Tracking passieren sollte (Habe ich mir vom Google AR Template abgeschaut)
  (if (`KismetSystemLibrary.IsValid` (`self.Pin`))
    (if (`|EnumEquality` (`ARPin.GetTrackingState` _pin) "Tracking")
      (`SceneComponent.K2_SetWorldTransform` (`self.WorldAnchorRoot`) (`ARPin.GetLocalToWorldTransform` _pin) false true))))

(fn `Set Cloud ID`
  (params (ID :type String))
  ;[0 1 0] Diese Funktion setzt die Cloud ID Variable die danach auf die Clients repliziert wird sodass die Clients die Anchor resolven können
  (`/Engine/EditorBlueprintResources/ActorMacros.Switch Has Authority`
    (:`Authority`
      (set `self.CloudID` ID))))

(fn `UserConstructionScript`)